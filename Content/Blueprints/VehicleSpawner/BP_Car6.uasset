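; BP_Car6 is a spawnable-style car actor that drives itself with a ProjectileMovement component and has switchable lights.
; Every Tick it adds a fixed amount to the current velocity's X and reapplies the result as local-space velocity, with no clamp in the graph.
; ToggleLighton and ToggleLightOff set a shared brightness value and apply it to two point lights and two spot lights.
; The construction script only calls the parent's.
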(event EventTick
  (params (DeltaSeconds :type Float%20%28single-precision%29))
  (bind _projectilemovement (Variables|Default|GetProjectileMovement))
  (bind _velocity (Variables|/Script/Engine.MovementComponent|GetVelocity _projectilemovement))
  (Game|Components|ProjectileMovement|SetVelocityinLocalSpace _projectilemovement (Math|Vector|MakeVector (+ 1e+01 (.x _velocity)) (.y _velocity) (.z _velocity))))

(event EventToggleLighton
  (Variables|Default|SetCurrentBrightness 5e+03)
  (Rendering|Components|Light|SetIntensity (Variables|Default|GetPointLight) (stale EventToggleLightOff _output_get)))

(event EventToggleLightOff
  (bind _output_get (Variables|Default|SetCurrentBrightness 0.0))
  (Rendering|Components|Light|SetIntensity (Variables|Default|GetPointLight) _output_get))

(fn ConstructionScript
  (|CallParentFunction))