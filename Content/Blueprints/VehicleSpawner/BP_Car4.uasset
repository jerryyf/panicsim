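; BP_Car4 is a vehicle Blueprint, filed under VehicleSpawner, with switchable lights and a hitbox that hurts the player.
; Custom events toggle two point lights and two spot lights, setting their shared intensity to either HeadlightBrightness or zero.
; A Box overlap applies a small amount of damage when the overlapping actor is the player pawn.
; The construction script only calls its parent.
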(event OnComponentBeginOverlap(Box)
  (params (OverlappedComponent :type Primitive%20Component%20Object%20Reference) (OtherActor :type Actor%20Object%20Reference) (OtherComp :type Primitive%20Component%20Object%20Reference) (OtherBodyIndex :type Integer) (bFromSweep :type Boolean) (SweepResult :type Hit%20Result%20Structure%20%28by%20ref%29))
  (bind _returnvalue (Game|Player|GetPlayerPawn 0))
  (if (== OtherActor _returnvalue)
    (Game|Damage|ApplyDamage _returnvalue 1.0 0 0)))

(event EventToggleLighton
  (Variables|Default|SetCurrentBrightness (Variables|Default|GetHeadlightBrightness))
  (Rendering|Components|Light|SetIntensity (Variables|Default|GetPointLight) (stale EventToggleLightOff _output_get)))

(event EventToggleLightOff
  (bind _output_get (Variables|Default|SetCurrentBrightness 0.0))
  (Rendering|Components|Light|SetIntensity (Variables|Default|GetPointLight) _output_get))

(fn ConstructionScript
  (|CallParentFunction))