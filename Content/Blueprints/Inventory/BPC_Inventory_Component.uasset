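; Inventory component that holds a fixed-size array of item slots, sized on BeginPlay, for the player's pickups and keys.
; AddToInventory fills partial stacks, then empty slots, looping on the leftover quantity, while unstackable items take one empty slot.
; ToggleInventory creates or removes a centre-anchored window on the first-person character's HUD canvas, switching cursor and input mode.
; UseKey removes a matching key's array element, shrinking the array; RefreshInventory is empty.
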(event EventBeginPlay
  (CallFunction|PrepareInventory))

(event EventTick
  (params (DeltaSeconds :type Float%20%28single-precision%29)))

(fn ToggleInventory
  (bind _returnvalue (Game|GetPlayerController 0))
  (bind _returnvalue_2 (Game|GetPlayerController 0))
  (bind _inventory_window (Variables|Default|GetInventory_Window)
    (:then
      (Widget|RemovefromParent _inventory_window)
      (Variables|Default|SetInventory_Window 0)
      (Input|SetInputModeGameOnly _returnvalue)
      (Variables|/Script/Engine.PlayerController|SetbShowMouseCursor _returnvalue false))
    (:else
      (bind _returnvalue_3 (UserInterface|CreateWidget "/Game/Blueprints/Inventory/InventoryUI/WBP_Inventory_Window.WBP_Inventory_Window_C" 0 self))
      (Variables|Default|SetInventory_Window _returnvalue_3)
      (bind _asbp_first_person_character (Utilities|Casting|CastToBP_FirstPersonCharacter (Game|Player|GetPlayerPawn 0)))
      (bind _returnvalue_4 (Class|CanvasPanel|AddChildtoCanvas (Variables|/Game/Blueprints/Inventory/InventoryUI/WBP_Inventory_HUD.WBP_Inventory_HUD_C|GetHUDCanvas (Variables|/Game/FirstPerson/Blueprints/BP_FirstPersonCharacter.BP_FirstPersonCharacter_C|GetHUD_Widget _asbp_first_person_character)) (Variables|Default|GetInventory_Window)))
      (Class|CanvasPanelSlot|SetAutoSize _returnvalue_4 true)
      (Class|CanvasPanelSlot|SetAlignment _returnvalue_4 "(X=0.500000,Y=0.500000)")
      (Class|CanvasPanelSlot|SetAnchors _returnvalue_4 (Utilities|Struct|MakeAnchors "(X=0.500000,Y=0.500000)" "(X=0.500000,Y=0.500000)"))
      (Class|CanvasPanelSlot|SetPosition _returnvalue_4 (Variables|Default|GetPosition))
      (Input|SetInputModeGameandUI _returnvalue_2 0 "LockAlways" true)
      (Variables|/Script/Engine.PlayerController|SetbShowMouseCursor _returnvalue_2 true))))

(fn AddtoInventory
  (params (PickUpItem :type BPS%20Slot%20Structure%20Structure))
  (bind (_itemstructure _quantity) (Utilities|Struct|BreakBPS_Slot_Structure PickUpItem))
  (bind _stackable (Utilities|Struct|BreakBPS_Item_Structure _itemstructure))
  (LocalVariables|SetLeftCount _quantity)
  (if (and (<= _quantity 0) _stackable)
    (return true 0)
    (else
      (if _stackable
        ;[1 1 1] Add Stackable Item
        (bind (_success _slotindex) (CallFunction|HasAvailableStack PickUpItem :!label _label))
        (if _success
          (bind _left (CallFunction|AddtoStack (Utilities|Struct|MakeBPS_Slot_Structure (.itemstructure PickUpItem) (LocalVariables|GetLeftCount)) _slotindex))
          (bind _output_get (LocalVariables|SetLeftCount _left))
          (LocalVariables|SetPicked true)
          (if (<= _output_get 0)
            (LocalVariables|SetSuccess true)
            (else
              (goto _label)))
          (elif (LocalVariables|GetPicked)
            (LocalVariables|SetSuccess true)
            (else
              (LocalVariables|SetSuccess false))))
        (else
          ;[1 1 1] Add unstackable Item
          (bind (_hasemptyslot _slotindex_2) (CallFunction|HasEmptySlot))
          (if _hasemptyslot
            (CallFunction|CreateNewStack (Utilities|Struct|MakeBPS_Slot_Structure (.itemstructure PickUpItem) 1) _slotindex_2)
            (LocalVariables|SetSuccess true)
            (LocalVariables|SetLeftCount 0)
            (else
              (LocalVariables|SetSuccess false)
              (LocalVariables|SetLeftCount 1)))))
      (return (LocalVariables|GetSuccess) (LocalVariables|GetLeftCount)))))

(fn PrepareInventory
  (Utilities|Array|Resize (Variables|Default|GetInventory) (Variables|Default|GetNumberOfSlots)))

(fn CreateNewStack
  (params (ContentToAdd :type BPS%20Slot%20Structure%20Structure) (SlotIndex :type Integer))
  (Utilities|Array|SetArrayElem (Variables|Default|GetInventory) SlotIndex ContentToAdd))

(fn AddtoStack
  (params (SlotStructure :type BPS%20Slot%20Structure%20Structure) (SlotIndex :type Integer))
  (bind (_itemstructure _quantity) (Utilities|Struct|BreakBPS_Slot_Structure SlotStructure))
  (bind _inventory (Variables|Default|GetInventory))
  (bind _maxstacksize (Utilities|Struct|BreakBPS_Item_Structure _itemstructure))
  (bind _output (Utilities|Array|Get(acopy) _inventory SlotIndex))
  (bind _returnvalue (+ _quantity (.quantity _output)))
  (LocalVariables|SetTotalQuantity _returnvalue)
  (Utilities|Array|SetArrayElem (Variables|Default|GetInventory) SlotIndex (Utilities|Struct|MakeBPS_Slot_Structure _itemstructure (Math|Integer|Min(Integer) _returnvalue _maxstacksize)))
  (return (Math|Integer|Max(Integer) (- (LocalVariables|GetTotalQuantity) _maxstacksize))))

(fn HasEmptySlot
  (bind _bps_slot_structure (Utilities|Struct|MakeBPS_Slot_Structure "(Name_6_0A0E11F64A0867EC5BCBBCAE403A1E09=\"\",Stackable_7_2AEA7D744F591E7B5A6DDA8B84CD7912=False,MaxStackSize_20_D96B25804AC22D68B73492AB52F51BC6=9,Thumbnail_13_B5FF234D4536BCD22C05ECBC91B96814=None,Description_14_FDC9AC76413B447C000A4A9CA13003A1=\"\",Consumable_18_A97111A245CF191B044AC4A15F18E4CB=True,Class_19_4437858E4CC346238B3157BDB28509A3=None,Type_27_079B897E484128A8292F45BF27409F67=NewEnumerator0,Key_Id_30_2F42716741F345470A41CE956CACE20A=0)"))
  (bind _inventory (Variables|Default|GetInventory))
  (bind _returnvalue (Utilities|Array|FindItem _inventory _bps_slot_structure))
  (return (not (== _returnvalue -1)) _returnvalue))

(fn HasAvailableStack
  (params (ItemToAdd :type BPS%20Slot%20Structure%20Structure))
  (bind _variable (|TemporaryVariable))
  (bind _variable_2 (|TemporaryVariable))
  ;[1 1 1] Find Unfullfilled Stack
  (bind (_array_element _array_index) (Utilities|Array|ForEachLoopwithBreak (Variables|Default|GetInventory) :!label _label)
    (:LoopBody
      (if (and (== (.Class (Utilities|Struct|BreakBPS_Item_Structure (.ItemStructure (Utilities|Struct|BreakBPS_Slot_Structure ItemToAdd)))) (.Class (Utilities|Struct|BreakBPS_Item_Structure (.ItemStructure (Utilities|Struct|BreakBPS_Slot_Structure _array_element))))) (< (.Quantity (Utilities|Struct|BreakBPS_Slot_Structure _array_element)) (.MaxStackSize (Utilities|Struct|BreakBPS_Item_Structure (.ItemStructure (Utilities|Struct|BreakBPS_Slot_Structure _array_element))))))
        (|Assign _variable_2 _array_index)
        (|Assign _variable true)
        (goto _label Break)))
    (:Completed
      (if _variable
        (LocalVariables|SetReturnBool true :!label _label_2)
        (else
          (bind (_hasemptyslot _slotindex) (CallFunction|HasEmptySlot))
          (if _hasemptyslot
            (|Assign _variable_2 _slotindex)
            (goto _label_2)
            (else
              (LocalVariables|SetReturnBool false)))))
      (return (LocalVariables|GetReturnBool) _variable_2))))

(fn RefreshInventory)

(fn ShowDescription
  (params (Content :type Text))
  (Variables|/Game/Blueprints/Inventory/InventoryUI/WBP_Inventory_Window.WBP_Inventory_Window_C|SetDescription (Variables|Default|GetInventory_Window) Content))

(fn UseKey
  (params (Key_Id :type Integer))
  (bind _inventory (Variables|Default|GetInventory))
  (bind (_array_element _array_index) (Utilities|Array|ForEachLoopwithBreak _inventory :!label _label)
    (:LoopBody
      (if (Utilities|Enum|Equal(Enum) (.Type (Utilities|Struct|BreakBPS_Item_Structure (.ItemStructure (Utilities|Struct|BreakBPS_Slot_Structure _array_element)))) "NewEnumerator1")
        (if (== (.Key_Id (Utilities|Struct|BreakBPS_Item_Structure (.ItemStructure (Utilities|Struct|BreakBPS_Slot_Structure _array_element)))) Key_Id)
          (Utilities|Array|RemoveIndex _inventory _array_index)
          (goto _label Break))))
    (:Completed
      (return (and (Utilities|Enum|Equal(Enum) (.Type (Utilities|Struct|BreakBPS_Item_Structure (.ItemStructure (Utilities|Struct|BreakBPS_Slot_Structure _array_element)))) "NewEnumerator1") (== (.Key_Id (Utilities|Struct|BreakBPS_Item_Structure (.ItemStructure (Utilities|Struct|BreakBPS_Slot_Structure _array_element)))) Key_Id))))))