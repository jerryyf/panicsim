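; Propane tank key item Blueprint for the inventory system, derived from a parent item class that provides highlight behavior.
; It overrides the highlight and remove-highlight functions, calling the parent and then swapping materials on its four static mesh components between normal and highlighted versions.
; The construction script only calls the parent, and the event graph holds no active logic.
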(event EventBeginPlay)

(event Collision|EventActorBeginOverlap
  (params (OtherActor :type Actor%20Object%20Reference)))

(event EventTick
  (params (DeltaSeconds :type Float%20%28single-precision%29)))

(fn ConstructionScript
  (|CallParentFunction))

(fn HighLight
  (|CallParentFunction)
  (Rendering|Material|SetMaterial (Variables|Default|GetStaticMesh) 0 "/Game/Blueprints/PickUpable/Propane_Tank/Material_Highlight.Material_Highlight")
  (Rendering|Material|SetMaterial (Variables|Default|GetStaticMesh1) 0 "/Game/Blueprints/PickUpable/Propane_Tank/Material_3_Hilight.Material_3_Hilight")
  (Rendering|Material|SetMaterial (Variables|Default|GetStaticMesh2) 0 "/Game/Blueprints/PickUpable/Propane_Tank/Material_2_Highlight.Material_2_Highlight")
  (Rendering|Material|SetMaterial (Variables|Default|GetStaticMesh3) 0 "/Game/Blueprints/PickUpable/Propane_Tank/Material_1_Highlight.Material_1_Highlight"))

(fn RemoveHightlight
  (|CallParentFunction)
  (Rendering|Material|SetMaterial (Variables|Default|GetStaticMesh) 0 "/Game/Blueprints/PickUpable/Propane_Tank/Material.Material")
  (Rendering|Material|SetMaterial (Variables|Default|GetStaticMesh1) 0 "/Game/Blueprints/PickUpable/Propane_Tank/Material_3.Material_3")
  (Rendering|Material|SetMaterial (Variables|Default|GetStaticMesh2) 0 "/Game/Blueprints/PickUpable/Propane_Tank/Material_2.Material_2")
  (Rendering|Material|SetMaterial (Variables|Default|GetStaticMesh3) 0 "/Game/Blueprints/PickUpable/Propane_Tank/Material_1.Material_1"))