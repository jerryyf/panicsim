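; Bottle inventory item that switches the first-person character's package type when used.
; Use succeeds only if the player has a different package type and is not being chased, then sets the type and calls PackageChange on the character; otherwise it returns a failure message.
; Highlight overrides call the parent, then swap the static mesh between normal and highlighted Crystal Geyser materials.
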(event EventBeginPlay)

(event Collision|EventActorBeginOverlap
  (params (OtherActor :type Actor%20Object%20Reference)))

(event EventTick
  (params (DeltaSeconds :type Float%20%28single-precision%29)))

(fn ConstructionScript
  (|CallParentFunction))

(fn HighLight
  (|CallParentFunction)
  (Rendering|Material|SetMaterial (Variables|Default|GetStaticMesh) 0 "/Game/StaticMeshes/Plastic_Bottle/CRYSTAL_GEYSER_Mat_HighLight.CRYSTAL_GEYSER_Mat_HighLight"))

(fn RemoveHightlight
  (|CallParentFunction)
  (Rendering|Material|SetMaterial (Variables|Default|GetStaticMesh) 0 "/Game/StaticMeshes/Plastic_Bottle/CRYSTAL_GEYSER_Mat.CRYSTAL_GEYSER_Mat"))

(fn UseItem
  (bind _asbp_first_person_character (Utilities|Casting|CastToBP_FirstPersonCharacter (Game|Player|GetPlayerPawn 0)))
  (if (Utilities|Enum|NotEqual(Enum) (Variables|/Game/FirstPerson/Blueprints/BP_FirstPersonCharacter.BP_FirstPersonCharacter_C|GetPackage_Type _asbp_first_person_character) "NewEnumerator0")
    (if (not (Default|IsBeingChased _asbp_first_person_character))
      (Variables|/Game/FirstPerson/Blueprints/BP_FirstPersonCharacter.BP_FirstPersonCharacter_C|SetPackage_Type _asbp_first_person_character "NewEnumerator0")
      (bind _asbp_first_person_character_2 (Utilities|Casting|CastToBP_FirstPersonCharacter (Game|Player|GetPlayerPawn 0)))
      (Default|PackageChange _asbp_first_person_character_2)
      (return true "")
      (else
        (return false "I can't change package now, its too dangerous.")))
    (else
      (return false "This is same to current package type, no need to change."))))