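; BP_Item_TinCan is a tin can package item that switches the first-person player character's package type when used.
; HighLight and RemoveHightlight extend the parent's versions by swapping materials on the can mesh and its separate lid.
; UseItem sets PackageType and calls PackageChange on the character, but fails with a warning message while the player is being chased.
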(fn ConstructionScript
  (|CallParentFunction))

(fn HighLight
  (bind _staticmesh (Variables|Default|GetStaticMesh))
  (|CallParentFunction)
  (Rendering|Material|SetMaterial _staticmesh 0 "/Game/StaticMeshes/Key/M_Highlighted_Key.M_Highlighted_Key")
  (Rendering|Material|SetMaterial _staticmesh 1 "/Game/StaticMeshes/Key/M_Highlighted_Key.M_Highlighted_Key")
  (Rendering|Material|SetMaterial (Variables|Default|GetLid) 0 "/Game/StaticMeshes/Tin_Can/blinn17_Highlight.blinn17_Highlight"))

(fn RemoveHightlight
  (bind _staticmesh (Variables|Default|GetStaticMesh))
  (|CallParentFunction)
  (Rendering|Material|SetMaterial _staticmesh 0 "/Game/StaticMeshes/Key/03_-_Default.03_-_Default")
  (Rendering|Material|SetMaterial _staticmesh 1 "/Game/StaticMeshes/Key/03_-_Default.03_-_Default")
  (Rendering|Material|SetMaterial (Variables|Default|GetLid) 0 "/Game/StaticMeshes/Key/03_-_Default.03_-_Default"))

(fn UseItem
  (bind _asbp_first_person_character (Utilities|Casting|CastToBP_FirstPersonCharacter (Game|Player|GetPlayerPawn 0)))
  (if (not (Default|IsBeingChased _asbp_first_person_character))
    (Variables|/Game/FirstPerson/Blueprints/BP_FirstPersonCharacter.BP_FirstPersonCharacter_C|SetPackage_Type _asbp_first_person_character "NewEnumerator1")
    (bind _asbp_first_person_character_2 (Utilities|Casting|CastToBP_FirstPersonCharacter (Game|Player|GetPlayerPawn 0)))
    (Default|PackageChange _asbp_first_person_character_2)
    (return true "")
    (else
      (return false "I can't change package now, its too dangerous. "))))