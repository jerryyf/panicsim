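; BP_Item_ChillPill is the Chill Pill inventory item, a child Blueprint that adds its own highlight visuals to inherited item behavior.
; HighLight and RemoveHightlight each call the parent, then swap materials between highlighted and normal variants on both StaticMesh slots and the Lid.
; The construction script only calls its parent.
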(fn ConstructionScript
  (|CallParentFunction))

(fn HighLight
  (bind _staticmesh (Variables|Default|GetStaticMesh))
  (|CallParentFunction)
  (Rendering|Material|SetMaterial _staticmesh 0 "/Game/StaticMeshes/Tin_Can/blinn17_Highlight.blinn17_Highlight")
  (Rendering|Material|SetMaterial _staticmesh 1 "/Game/StaticMeshes/Tin_Can/blinn15_Highlight.blinn15_Highlight")
  (Rendering|Material|SetMaterial (Variables|Default|GetLid) 0 "/Game/StaticMeshes/Tin_Can/blinn17_Highlight.blinn17_Highlight"))

(fn RemoveHightlight
  (bind _staticmesh (Variables|Default|GetStaticMesh))
  (|CallParentFunction)
  (Rendering|Material|SetMaterial _staticmesh 0 "/Game/StaticMeshes/Tin_Can/blinn17.blinn17")
  (Rendering|Material|SetMaterial _staticmesh 1 "/Game/StaticMeshes/Tin_Can/blinn15.blinn15")
  (Rendering|Material|SetMaterial (Variables|Default|GetLid) 0 "/Game/StaticMeshes/Tin_Can/blinn17.blinn17"))