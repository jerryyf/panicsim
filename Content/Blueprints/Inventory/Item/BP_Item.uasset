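; BP_Item is a world pickup actor carrying an item struct and quantity that the player can collect into an inventory.
; Look events refresh the WBP_Item_Info count plate and show it with a pickup notice only within pickup range, measured as Manhattan distance.
; Interacting while highlighted adds to the interactor's BPC_Inventory_Component, plays a sound, then destroys the actor or keeps the leftover quantity.
; UseItem is a stub returning failure.
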(event EventLookingat
  (CallFunction|UpdateCount (Variables|Default|GetQuantity))
  (CallFunction|UpdateName (.name (Variables|Default|GetItem_Structure)))
  (if (CallFunction|WithinPickUpDistance (Variables|Default|GetPickUpDistance))
    (CallFunction|HighLight)
    (Variables|Default|SetHighlighted true)
    (else
      (CallFunction|RemoveHightlight)
      (Variables|Default|SetHighlighted false))))

(event EventLookAway
  (CallFunction|UpdateCount (Variables|Default|GetQuantity))
  (CallFunction|UpdateName (.name (Variables|Default|GetItem_Structure)))
  (CallFunction|RemoveHightlight)
  (Variables|Default|SetHighlighted false))

(event EventInteract
  (params (Interactor :type Actor%20Object%20Reference))
  (if (Variables|Default|GetHighlighted)
    (bind (_added _left) (Default|AddtoInventory (Actor|GetComponentbyClass Interactor "/Game/Blueprints/Inventory/BPC_Inventory_Component.BPC_Inventory_Component_C") (Utilities|Struct|MakeBPS_Slot_Structure (Variables|Default|GetItem_Structure) (Variables|Default|GetQuantity))))
    (if _added
      (Audio|PlaySoundatLocation (Variables|Default|GetPickUpSound) (.location (Transformation|GetActorTransform)) "0, 0, 0" 1.0 1.0 0.0 0 0 0 0)
      (if (<= _left 0)
        (Actor|DestroyActor)
        (else
          (bind _output_get (Variables|Default|SetQuantity _left))
          (CallFunction|UpdateCount _output_get))))))

(fn ConstructionScript)

(fn WithinPickUpDistance
  (params (PickUpDistance :type Float%20%28double-precision%29))
  (return (<= (Math|Vector|DotProduct (Math|Vector|VectorGetAbs (- (Transformation|GetActorLocation (Game|Player|GetPlayerPawn 0)) (Transformation|GetActorLocation))) "1.000000,1.000000,1.000000") PickUpDistance)))

(fn HighLight
  (Rendering|SetVisibility (Variables|Default|GetPickUp_Notice) true false))

(fn RemoveHightlight
  (Rendering|SetVisibility (Variables|Default|GetPickUp_Notice) false false))

(fn UpdateCount
  (params (NewCount :type Integer))
  (bind _aswbp_item_info (Utilities|Casting|CastToWBP_Item_Info (UserInterface|GetWidget (Variables|Default|GetCountPlate))))
  (Variables|/Game/Blueprints/PickUpable/WBP_Item_Info.WBP_Item_Info_C|SetQuantity _aswbp_item_info NewCount))

(fn UpdateName
  (params (NewName :type Name))
  (bind _aswbp_item_info (Utilities|Casting|CastToWBP_Item_Info (UserInterface|GetWidget (Variables|Default|GetCountPlate))))
  (Variables|/Game/Blueprints/PickUpable/WBP_Item_Info.WBP_Item_Info_C|SetName _aswbp_item_info NewName))

(fn UseItem
  (return false ""))