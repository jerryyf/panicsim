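; BP_Item_CalmPill is a calm pill inventory item that raises the first-person character's maximum panic value when used.
; It extends a parent item's highlight functions, swapping materials on the bottle mesh and lid between highlighted and normal versions.
; UseItem casts the player pawn to BP_FirstPersonCharacter, adds a fixed amount to MaxPanicValue rather than changing current panic, and returns true.
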(fn ConstructionScript
  (|CallParentFunction))

(fn HighLight
  (bind _staticmesh (Variables|Default|GetStaticMesh))
  (|CallParentFunction)
  (Rendering|Material|SetMaterial _staticmesh 0 "/Game/StaticMeshes/Calm_Pill/Calm_Pill_Banner_Highlighted.Calm_Pill_Banner_Highlighted")
  (Rendering|Material|SetMaterial _staticmesh 1 "/Game/StaticMeshes/Chill_Pill/pill_edge_highlighted.pill_edge_highlighted")
  (Rendering|Material|SetMaterial _staticmesh 2 "/Game/StaticMeshes/Chill_Pill/pill_bottle_highlighted.pill_bottle_highlighted")
  (Rendering|Material|SetMaterial (Variables|Default|GetLid) 0 "/Game/StaticMeshes/Chill_Pill/pill_edge_highlighted.pill_edge_highlighted"))

(fn RemoveHightlight
  (bind _staticmesh (Variables|Default|GetStaticMesh))
  (|CallParentFunction)
  (Rendering|Material|SetMaterial _staticmesh 0 "/Game/StaticMeshes/Calm_Pill/Calm_Pill_Banner.Calm_Pill_Banner")
  (Rendering|Material|SetMaterial _staticmesh 1 "/Game/StaticMeshes/Chill_Pill/pill_edge.pill_edge")
  (Rendering|Material|SetMaterial _staticmesh 2 "/Game/StaticMeshes/Chill_Pill/pill_bottle.pill_bottle")
  (Rendering|Material|SetMaterial (Variables|Default|GetLid) 0 "/Game/StaticMeshes/Chill_Pill/pill_edge.pill_edge"))

(fn UseItem
  (bind _asbp_first_person_character (Utilities|Casting|CastToBP_FirstPersonCharacter (Game|Player|GetPlayerPawn 0)))
  (Variables|/Game/FirstPerson/Blueprints/BP_FirstPersonCharacter.BP_FirstPersonCharacter_C|SetMax_Panic_Value _asbp_first_person_character (+ (Variables|/Game/FirstPerson/Blueprints/BP_FirstPersonCharacter.BP_FirstPersonCharacter_C|GetMax_Panic_Value _asbp_first_person_character) 3e+01))
  (return true))