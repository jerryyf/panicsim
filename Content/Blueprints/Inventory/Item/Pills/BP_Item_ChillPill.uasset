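; BP_Item_ChillPill is an inventory item, a pill bottle that lowers the first-person character's panic when used.
; UseItem subtracts a fixed amount from PanicValue, or fails with a message, resetting it to zero, when the player is not panicking.
; Highlight overrides extend the parent's behavior by swapping the bottle mesh and lid between normal and highlighted materials.
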(fn ConstructionScript
  (|CallParentFunction))

(fn HighLight
  (bind _staticmesh (Variables|Default|GetStaticMesh))
  (|CallParentFunction)
  (Rendering|Material|SetMaterial _staticmesh 0 "/Game/StaticMeshes/Chill_Pill/pill_banner_highlighted.pill_banner_highlighted")
  (Rendering|Material|SetMaterial _staticmesh 1 "/Game/StaticMeshes/Chill_Pill/pill_edge_highlighted.pill_edge_highlighted")
  (Rendering|Material|SetMaterial _staticmesh 2 "/Game/StaticMeshes/Chill_Pill/pill_bottle_highlighted.pill_bottle_highlighted")
  (Rendering|Material|SetMaterial (Variables|Default|GetLid) 0 "/Game/StaticMeshes/Chill_Pill/pill_edge_highlighted.pill_edge_highlighted"))

(fn RemoveHightlight
  (bind _staticmesh (Variables|Default|GetStaticMesh))
  (|CallParentFunction)
  (Rendering|Material|SetMaterial _staticmesh 0 "/Game/StaticMeshes/Chill_Pill/pill_banner.pill_banner")
  (Rendering|Material|SetMaterial _staticmesh 1 "/Game/StaticMeshes/Chill_Pill/pill_edge.pill_edge")
  (Rendering|Material|SetMaterial _staticmesh 2 "/Game/StaticMeshes/Chill_Pill/pill_bottle.pill_bottle")
  (Rendering|Material|SetMaterial (Variables|Default|GetLid) 0 "/Game/StaticMeshes/Chill_Pill/pill_edge.pill_edge"))

(fn UseItem
  (bind _asbp_first_person_character (Utilities|Casting|CastToBP_FirstPersonCharacter (Game|Player|GetPlayerPawn 0)))
  (if (<= (Variables|/Game/FirstPerson/Blueprints/BP_FirstPersonCharacter.BP_FirstPersonCharacter_C|GetPanic_Value _asbp_first_person_character) 0.0)
    (Variables|/Game/FirstPerson/Blueprints/BP_FirstPersonCharacter.BP_FirstPersonCharacter_C|SetPanic_Value _asbp_first_person_character 0.0)
    (return false "You are not panicking, don't waste the pills")
    (else
      (Variables|/Game/FirstPerson/Blueprints/BP_FirstPersonCharacter.BP_FirstPersonCharacter_C|SetPanic_Value _asbp_first_person_character (- (Variables|/Game/FirstPerson/Blueprints/BP_FirstPersonCharacter.BP_FirstPersonCharacter_C|GetPanic_Value _asbp_first_person_character) 3e+01))
      (return true ""))))