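; Win_Box is a trigger volume that plays the win sequence when the player reaches it.
; Its box overlap passes through a DoOnce before checking for player pawn 0, so the first overlap by any actor consumes the trigger.
; For the player, it switches the view to BP_Camera_Ending, plays a car driving-away sound, calls Spawn on BP_VehicleSpawner2 and shows the WBP_YouWin widget.
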(event OnComponentBeginOverlap(Box)
  (params (OverlappedComponent :type Primitive%20Component%20Object%20Reference) (OtherActor :type Actor%20Object%20Reference) (OtherComp :type Primitive%20Component%20Object%20Reference) (OtherBodyIndex :type Integer) (bFromSweep :type Boolean) (SweepResult :type Hit%20Result%20Structure%20%28by%20ref%29))
  (Utilities|FlowControl|DoOnce false
    (:Completed
      (if (== OtherActor (Game|Player|GetPlayerPawn 0))
        (bind _returnvalue (Actor|GetActorOfClass "/Game/Blueprints/BP_Camera_Ending.BP_Camera_Ending_C"))
        (Game|Player|SetViewTargetwithBlend (Game|GetPlayerController 0) _returnvalue 0.0 "VTBlend_Linear" 0.0 false)
        (Audio|PlaySound2D "/Game/Audio/car_driving_away.car_driving_away" 1.0 1.0 0.0 0 0)
        (bind _returnvalue_2 (Actor|GetActorOfClass "/Game/Blueprints/VehicleSpawner/BP_VehicleSpawner2.BP_VehicleSpawner2_C"))
        (Default|Spawn _returnvalue_2)
        (bind _returnvalue_3 (UserInterface|CreateWidget "/Game/Blueprints/UI/GameMenu/WBP_YouWin.WBP_YouWin_C"))
        (UserInterface|Viewport|AddtoViewport _returnvalue_3 0)))))

(fn ConstructionScript)