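; Level trigger actor that destroys a list of actors when the player pawn overlaps it.
; BeginPlay disables collision on Box1, and the trigger re-enables it with query and physics after destroying every entry in ActorList.
; A DoOnce precedes the player check, so the first overlap of any actor uses up the trigger, even if it is not the player.
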(event Collision|EventActorBeginOverlap
  (params (OtherActor :type Actor%20Object%20Reference))
  (Utilities|FlowControl|DoOnce false
    (:Completed
      (if (== OtherActor (Game|Player|GetPlayerPawn 0))
        (for _array_element (Variables|Default|GetActorList)
          (Actor|DestroyActor _array_element))
        (Collision|SetCollisionEnabled (Variables|Default|GetBox1) "QueryAndPhysics")))))

(event EventBeginPlay
  (Collision|SetCollisionEnabled (Variables|Default|GetBox1) "NoCollision"))

(fn ConstructionScript)