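; BP_TriggerMessageOnce is a level trigger that shows a message on screen once, for a set duration.
; On begin overlap it passes a DoOnce gate, then creates a WDJ_Message widget with its Message text if the overlapping actor is the player pawn.
; The widget is removed after a Delay of Duration.
; The gate precedes the player check, so any actor's first overlap uses up the trigger.
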(event Collision|EventActorBeginOverlap
  (params (OtherActor :type Actor%20Object%20Reference))
  (Utilities|FlowControl|DoOnce false
    (:Completed
      (if (== OtherActor (Game|Player|GetPlayerPawn 0))
        (bind _returnvalue (UserInterface|CreateWidget "/Game/Blueprints/Door/WDJ_Message.WDJ_Message_C"))
        (Variables|/Game/Blueprints/Door/WDJ_Message.WDJ_Message_C|SetMessage _returnvalue (Variables|Default|GetMessage))
        (UserInterface|Viewport|AddtoViewport _returnvalue 0)
        (Utilities|FlowControl|Delay (Variables|Default|GetDuration))
        (Widget|RemovefromParent _returnvalue)))))

(fn ConstructionScript)