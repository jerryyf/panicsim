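; BP_Trigger_Message_Box is a trigger volume that shows a text message on screen while the player stands inside it.
; When the player pawn begins overlapping the Box, it creates a WDJ_Message widget, passes it the Message variable and adds it to the viewport.
; End overlap by the player removes the widget and clears the Overlap flag, which any actor entering sets.
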(event OnComponentBeginOverlap(Box)
  (params (OverlappedComponent :type Primitive%20Component%20Object%20Reference) (OtherActor :type Actor%20Object%20Reference) (OtherComp :type Primitive%20Component%20Object%20Reference) (OtherBodyIndex :type Integer) (bFromSweep :type Boolean) (SweepResult :type Hit%20Result%20Structure%20%28by%20ref%29))
  (Variables|Default|SetOverlap true)
  (if (== OtherActor (Game|Player|GetPlayerPawn 0))
    (bind _returnvalue (UserInterface|CreateWidget "/Game/Blueprints/Door/WDJ_Message.WDJ_Message_C"))
    (Variables|/Game/Blueprints/Door/WDJ_Message.WDJ_Message_C|SetMessage _returnvalue (Variables|Default|GetMessage))
    (UserInterface|Viewport|AddtoViewport _returnvalue 0)))

(event OnComponentEndOverlap(Box)
  (params (OverlappedComponent :type Primitive%20Component%20Object%20Reference) (OtherActor :type Actor%20Object%20Reference) (OtherComp :type Primitive%20Component%20Object%20Reference) (OtherBodyIndex :type Integer))
  (if (== OtherActor (Game|Player|GetPlayerPawn 0))
    (Variables|Default|SetOverlap false)
    (Widget|RemovefromParent (stale OnComponentBeginOverlap(Box) _returnvalue))))

(fn ConstructionScript)