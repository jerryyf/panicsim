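; Interactable fence door that the player can swing open when nearby, with an on-screen notice while it is still closed.
; HighLight checks the player's Manhattan distance against InteractionDistance to show the notice and set IsPlayerNearby; RemoveHighLight clears both.
; PickUp, gated by IsPlayerNearby, plays the Open timeline to drive the Door's relative pitch, marks it Opened and hides the notice.
; No closing logic exists, and the collision-disable node is unconnected.
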(event EventHighLight
  (if (CallFunction|WithinInteractionDistance (Variables|Default|GetInteraction_Distance))
    (if (not (Variables|Default|GetOpened))
      (Rendering|SetVisibility (Variables|Default|GetOpenDoorNotice) true false)
      (Variables|Default|SetIs_Player_Nearby true))
    (else
      (Rendering|SetVisibility (Variables|Default|GetOpenDoorNotice) false false)
      (Variables|Default|SetIs_Player_Nearby false))))

(event EventRemoveHighLight
  (Rendering|SetVisibility (Variables|Default|GetOpenDoorNotice) false false)
  (Variables|Default|SetIs_Player_Nearby false))

(event EventPickUp
  (bind _door (Variables|Default|GetDoor))
  (bind _returnvalue (Transformation|GetRelativeTransform _door))
  (if (Variables|Default|GetIs_Player_Nearby)
    (bind _open (Timeline|Open Play)
      (:Update
        (Transformation|SetRelativeLocationAndRotation (Variables|Default|GetDoor) (.location _returnvalue) (Math|Rotator|MakeRotator (.roll (.rotation _returnvalue)) _open (.yaw (.rotation _returnvalue))) false false)
        (Variables|Default|SetOpened true)
        (Rendering|SetVisibility (Variables|Default|GetOpenDoorNotice) false false)))))

(fn ConstructionScript)

(fn WithinInteractionDistance
  (params (Distance :type Float%20%28double-precision%29))
  (return (<= (Math|Vector|DotProduct (Math|Vector|VectorGetAbs (- (Transformation|GetActorLocation (Game|Player|GetPlayerPawn 0)) (Transformation|GetActorLocation))) "1.000000,1.000000,1.000000") Distance)))