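; BP_DDoor2 is an interactable double door that the player opens once, with a sound.
; HighLight and RemoveHighLight toggle the open prompt and nearby flag, using a summed per-axis distance to the player pawn rather than straight-line distance.
; PickUp, when the player is flagged nearby, plays a timeline that yaws both doors, sets Opened and hides the prompt.
; The node disabling door collision is unconnected.
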(event EventHighLight
  (if (CallFunction|WithinInteractionDistance (Variables|Default|GetInteraction_Distance))
    (if (not (Variables|Default|GetOpened))
      (Rendering|SetVisibility (Variables|Default|GetOpenDoorNotice) true false)
      (Variables|Default|SetIs_Player_Nearby true))
    (else
      (Rendering|SetVisibility (Variables|Default|GetOpenDoorNotice) false false)
      (Variables|Default|SetIs_Player_Nearby false))))

(event EventRemoveHighLight
  (Rendering|SetVisibility (Variables|Default|GetOpenDoorNotice) false false)
  (Variables|Default|SetIs_Player_Nearby false))

(event EventPickUp
  (bind _door (Variables|Default|GetDoor))
  (bind _door1 (Variables|Default|GetDoor1))
  (bind _returnvalue (Transformation|GetRelativeTransform _door))
  (bind _returnvalue_2 (Transformation|GetRelativeTransform _door1))
  (if (Variables|Default|GetIs_Player_Nearby)
    (Audio|PlaySound2D "/Game/Audio/door_open2.door_open2" 1.0 1.0 0.0 0 0)
    (bind (_direction _open _open2) (Timeline|Open Play)
      (:Update
        (Transformation|SetRelativeLocationAndRotation (Variables|Default|GetDoor) (.location _returnvalue) (Math|Rotator|MakeRotator (.roll (.rotation _returnvalue)) (.pitch (.rotation _returnvalue)) _open) false false)
        (Transformation|SetRelativeLocationAndRotation (Variables|Default|GetDoor1) (.location _returnvalue_2) (Math|Rotator|MakeRotator (.roll (.rotation _returnvalue_2)) (.pitch (.rotation _returnvalue_2)) _open2) false false)
        (Variables|Default|SetOpened true)
        (Rendering|SetVisibility (Variables|Default|GetOpenDoorNotice) false false)))))

(fn ConstructionScript)

(fn WithinInteractionDistance
  (params (Distance :type Float%20%28double-precision%29))
  (return (<= (Math|Vector|DotProduct (Math|Vector|VectorGetAbs (- (Transformation|GetActorLocation (Game|Player|GetPlayerPawn 0)) (Transformation|GetActorLocation))) "1.000000,1.000000,1.000000") Distance)))