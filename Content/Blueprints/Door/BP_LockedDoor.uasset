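; BP_LockedDoor is a door that opens only when the player carries a key matching its DoorId.
; HighLight and RemoveHighLight toggle the open prompt and nearby flag, with range measured as a Manhattan distance to the player pawn.
; PickUp calls CheckKeys, which removes the matching key from BP_FirstPersonCharacterDiff to unlock.
; An unlocked door drops collision and swings its yaw on a Timeline, otherwise a locked notice shows briefly.
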(event EventHighLight
  (if (CallFunction|WithinInteractionDistance (Variables|Default|GetInteraction_Distance))
    (if (not (Variables|Default|GetOpened))
      (Rendering|SetVisibility (Variables|Default|GetOpenDoorNotice) true false)
      (Variables|Default|SetIs_Player_Nearby true))
    (else
      (Rendering|SetVisibility (Variables|Default|GetOpenDoorNotice) false false)
      (Variables|Default|SetIs_Player_Nearby false))))

(event EventRemoveHighLight
  (Rendering|SetVisibility (Variables|Default|GetOpenDoorNotice) false false)
  (Variables|Default|SetIs_Player_Nearby false))

(event EventPickUp
  (bind _door (Variables|Default|GetDoor))
  (bind _doorlockednotice (Variables|Default|GetDoorLockedNotice))
  (bind _returnvalue (Transformation|GetRelativeTransform _door))
  (if (Variables|Default|GetIs_Player_Nearby)
    (Variables|Default|SetAttemped true)
    (CallFunction|CheckKeys)
    (if (Variables|Default|GetUnlocked)
      (Collision|SetCollisionEnabled (Variables|Default|GetDoor_Collision) "NoCollision")
      (bind _open (Timeline|Open Play)
        (:Update
          (Transformation|SetRelativeLocationAndRotation (Variables|Default|GetDoor) (.location _returnvalue) (Math|Rotator|MakeRotator (.roll (.rotation _returnvalue)) (.pitch (.rotation _returnvalue)) _open) false false)
          (Variables|Default|SetOpened true)
          (Rendering|SetVisibility (Variables|Default|GetOpenDoorNotice) false false)))
      (else
        (Rendering|SetVisibility _doorlockednotice true false)
        (Utilities|FlowControl|Delay 1.0)
        (Rendering|SetVisibility _doorlockednotice false false)))))

(fn ConstructionScript)

(fn WithinInteractionDistance
  (params (Distance :type Float%20%28double-precision%29))
  (return (<= (Math|Vector|DotProduct (Math|Vector|VectorGetAbs (- (Transformation|GetActorLocation (Game|Player|GetPlayerPawn 0)) (Transformation|GetActorLocation))) "1.000000,1.000000,1.000000") Distance)))

(fn CheckKeys
  (bind _asbp_first_person_character (Utilities|Casting|CastToBP_FirstPersonCharacterDiff (Game|Player|GetPlayerPawn 0)))
  (bind _array_element (Utilities|Array|ForEachLoopwithBreak (Variables|/Game/FirstPerson/Blueprints/BP_FirstPersonCharacterDiff.BP_FirstPersonCharacterDiff_C|GetKeys _asbp_first_person_character) :!label _label)
    (:LoopBody
      (if (== (Variables|Default|GetDoor_Id) _array_element)
        (bind _returnvalue (Utilities|Array|RemoveItem (Variables|/Game/FirstPerson/Blueprints/BP_FirstPersonCharacterDiff.BP_FirstPersonCharacterDiff_C|GetKeys _asbp_first_person_character) _array_element))
        (Variables|Default|SetUnlocked _returnvalue)
        (goto _label Break)))))