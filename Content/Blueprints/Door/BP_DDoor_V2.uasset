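; Lockable double door that the player toggles on interaction and that opens automatically when an Enemy_NPC enters its sphere.
; A timeline swings both leaves, with direction chosen by comparing the door's forward vector to the opener's relative position.
; Interaction checks the player's keys for DoorId, consuming a match or showing a timed locked message.
; Highlight events display a distance-gated prompt widget, while construction and SetDoor apply the mesh and open state.
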(event OnComponentBeginOverlap(Sphere)
  (params (OverlappedComponent :type Primitive%20Component%20Object%20Reference) (OtherActor :type Actor%20Object%20Reference) (OtherComp :type Primitive%20Component%20Object%20Reference) (OtherBodyIndex :type Integer) (bFromSweep :type Boolean) (SweepResult :type Hit%20Result%20Structure%20%28by%20ref%29))
  (bind _returnvalue (Transformation|GetActorLocation))
  (bind _door1 (Variables|Default|GetDoor1))
  (bind _door (Variables|Default|GetDoor))
  (if (== (Utilities|GetClass OtherActor) "/Game/AI/Enemy/Enemy_NPC.Enemy_NPC_C")
    (Variables|Default|SetOverlapping true)
    (if (not (Variables|Default|GetOpened))
      (Audio|PlaySoundatLocation (Variables|Default|GetOpenDoorSound) (Transformation|GetActorLocation) "0, 0, 0" 1.0 1.0 0.0 "/Game/Audio/NewSoundAttenuation.NewSoundAttenuation" 0 0 0)
      (Variables|Default|SetOpened true)
      (Variables|Default|SetDirection (Utilities|Operators|EqualEqual (Transformation|GetActorForwardVector) (Math|Vector|Normalize (- (Transformation|GetActorLocation OtherActor) (Transformation|GetActorLocation))) 1.0))
      ;[1 1 1] Open Door and Check Key
      (bind (_direction _open _open2) (Timeline|Timeline_0 PlayFromStart)
        (:Update
          (if (Variables|Default|GetDirection)
            (Variables|Default|SetOpenDirection false)
            (else
              (Variables|Default|SetOpenDirection true)))
          (Transformation|SetRelativeLocationAndRotation _door (Variables|/Script/Engine.SceneComponent|GetRelativeLocation _door) (Math|Rotator|MakeRotator 0.0 0.0 (* _open 1.0 (Math|Float|SelectFloat 1.0 -1.0 (Variables|Default|GetDirection)))) false false)
          (Transformation|SetRelativeLocationAndRotation _door1 (Variables|/Script/Engine.SceneComponent|GetRelativeLocation _door1) (Math|Rotator|MakeRotator 0.0 0.0 (* _open2 1.0 (Math|Float|SelectFloat 1.0 -1.0 (Variables|Default|GetDirection)))) false false))
        (:Finished
          (Utilities|FlowControl|DoOnce false) ; enters at Reset
        )))))

(event OnComponentEndOverlap(Sphere)
  (params (OverlappedComponent :type Primitive%20Component%20Object%20Reference) (OtherActor :type Actor%20Object%20Reference) (OtherComp :type Primitive%20Component%20Object%20Reference) (OtherBodyIndex :type Integer))
  (if (== (Utilities|GetClass OtherActor) "/Game/AI/Enemy/Enemy_NPC.Enemy_NPC_C")
    (Variables|Default|SetOverlapping false)))

(event Custom|OpenDoor
  (bind _returnvalue (Transformation|GetActorLocation))
  (bind _door1 (Variables|Default|GetDoor1))
  (bind _door (Variables|Default|GetDoor))
  (if (not (Variables|Default|GetOpened))
    (Audio|PlaySoundatLocation (Variables|Default|GetOpenDoorSound) (Transformation|GetActorLocation) "0, 0, 0" 1.0 1.0 0.0 "/Game/Audio/NewSoundAttenuation.NewSoundAttenuation" 0 0 0)
    (Variables|Default|SetOpened true)
    (Variables|Default|SetDirection (Utilities|Operators|EqualEqual (Transformation|GetActorForwardVector) (Math|Vector|Normalize (- (Transformation|GetActorLocation (stale OnComponentBeginOverlap(Sphere) OtherActor)) (Transformation|GetActorLocation))) 1.0))
    ;[1 1 1] Open Door and Check Key
    (bind (_direction _open _open2) (Timeline|Timeline_0 PlayFromStart)
      (:Update
        (if (Variables|Default|GetDirection)
          (Variables|Default|SetOpenDirection false)
          (else
            (Variables|Default|SetOpenDirection true)))
        (Transformation|SetRelativeLocationAndRotation _door (Variables|/Script/Engine.SceneComponent|GetRelativeLocation _door) (Math|Rotator|MakeRotator 0.0 0.0 (* _open 1.0 (Math|Float|SelectFloat 1.0 -1.0 (Variables|Default|GetDirection)))) false false)
        (Transformation|SetRelativeLocationAndRotation _door1 (Variables|/Script/Engine.SceneComponent|GetRelativeLocation _door1) (Math|Rotator|MakeRotator 0.0 0.0 (* _open2 1.0 (Math|Float|SelectFloat 1.0 -1.0 (Variables|Default|GetDirection)))) false false))
      (:Finished
        (Utilities|FlowControl|DoOnce false) ; enters at Reset
      ))))

(event EventTick
  (params (DeltaSeconds :type Float%20%28single-precision%29))
  (Variables|Default|SetWithinInteractionDistance (CallFunction|WithinInteractionDistance (Variables|Default|GetInteraction_Distance)))
  (if (Variables|Default|GetOverlapping)
    (CallFunction|OpenDoor)))

(event EventHighLight
  ;[1 1 1] Show Door Prompt
  (if (Variables|Default|GetWithinInteractionDistance)
    (Rendering|SetVisibility (Variables|Default|GetOpenDoorNotice) true false)
    (bind _returnvalue (UserInterface|CreateWidget "/Game/Blueprints/Door/WBP_OpenDoor.WBP_OpenDoor_C"))
    (if (Variables|Default|GetDisplayLocked)
      (Variables|/Game/Blueprints/Door/WBP_OpenDoor.WBP_OpenDoor_C|SetPrompt _returnvalue "Locked")
      (elif (Variables|Default|GetOpened)
        (Variables|/Game/Blueprints/Door/WBP_OpenDoor.WBP_OpenDoor_C|SetPrompt _returnvalue "Close Door [E]")
        (else
          (Variables|/Game/Blueprints/Door/WBP_OpenDoor.WBP_OpenDoor_C|SetPrompt _returnvalue "Open Door [E]"))))
    (UserInterface|SetWidget (Variables|Default|GetOpenDoorNotice) _returnvalue)
    (Variables|Default|SetIs_Player_Nearby true)
    (else
      (Rendering|SetVisibility (Variables|Default|GetOpenDoorNotice) false false)
      (Variables|Default|SetIs_Player_Nearby false))))

(event EventRemoveHighLight
  ;[1 1 1] Show Door Prompt
  (Rendering|SetVisibility (Variables|Default|GetOpenDoorNotice) false false)
  (Variables|Default|SetIs_Player_Nearby false))

(event EventPickUp
  (bind _returnvalue (Transformation|GetActorLocation))
  (bind _door1 (Variables|Default|GetDoor1))
  (bind _door (Variables|Default|GetDoor))
  ;[1 1 1] Open Door and Check Key
  (if (Variables|Default|GetIs_Player_Nearby)
    (if (Variables|Default|GetUnlocked)
      (Utilities|FlowControl|DoOnce false :!label _label
        (:Completed
          _))
      (else
        (CallFunction|CheckKeys)
        (if (Variables|Default|GetUnlocked)
          (Audio|PlaySoundatLocation (Variables|Default|GetUnlockDoorSound) _returnvalue "0, 0, 0" 1.0 1.0 0.0 "/Game/Audio/NewSoundAttenuation.NewSoundAttenuation" 0 0 0)
          (else
            ;[1 1 1] Handle Locked Prompts
            (Utilities|FlowControl|DoOnce false :!label _label_2
              (:Completed
                (Variables|Default|SetDisplayLocked true)
                (bind _returnvalue_2 (UserInterface|CreateWidget "/Game/Blueprints/Door/WDJ_Message.WDJ_Message_C"))
                (Variables|/Game/Blueprints/Door/WDJ_Message.WDJ_Message_C|SetMessage _returnvalue_2 (Variables|Default|GetDoor%20Locked%20Message))
                (UserInterface|Viewport|AddtoViewport _returnvalue_2 0)
                (Audio|PlaySoundatLocation (Variables|Default|GetLockedDoorSound) (Transformation|GetActorLocation) "0, 0, 0" 1.0 1.0 0.0 "/Game/Audio/NewSoundAttenuation.NewSoundAttenuation" 0 0 0)
                (Utilities|FlowControl|Delay 2.0)
                (Widget|RemovefromParent _returnvalue_2)
                (Variables|Default|SetDisplayLocked false)
                (goto _label_2 Reset)))))))
    (if (Variables|Default|GetOpened)
      (Audio|PlaySoundatLocation (Variables|Default|GetCloseDoorSound) _returnvalue "0, 0, 0" 1.0 1.0 0.0 "/Game/Audio/NewSoundAttenuation.NewSoundAttenuation" 0 0 0)
      (Variables|Default|SetOpened false)
      (bind (_direction _open _open2) (Timeline|Timeline_0 ReverseFromEnd)
        (:Update
          (if (Variables|Default|GetDirection)
            (Variables|Default|SetOpenDirection false)
            (else
              (Variables|Default|SetOpenDirection true)))
          (Transformation|SetRelativeLocationAndRotation _door (Variables|/Script/Engine.SceneComponent|GetRelativeLocation _door) (Math|Rotator|MakeRotator 0.0 0.0 (* _open 1.0 (Math|Float|SelectFloat 1.0 -1.0 (Variables|Default|GetDirection)))) false false)
          (Transformation|SetRelativeLocationAndRotation _door1 (Variables|/Script/Engine.SceneComponent|GetRelativeLocation _door1) (Math|Rotator|MakeRotator 0.0 0.0 (* _open2 1.0 (Math|Float|SelectFloat 1.0 -1.0 (Variables|Default|GetDirection)))) false false))
        (:Finished
          (goto _label Reset)))
      (else
        (Audio|PlaySoundatLocation (Variables|Default|GetOpenDoorSound) _returnvalue "0, 0, 0" 1.0 1.0 0.0 "/Game/Audio/NewSoundAttenuation.NewSoundAttenuation" 0 0 0)
        (Variables|Default|SetOpened true)
        (Variables|Default|SetDirection (Utilities|Operators|EqualEqual (Transformation|GetActorForwardVector) (Math|Vector|Normalize (- (Transformation|GetActorLocation (Game|Player|GetPlayerPawn 0)) (Transformation|GetActorLocation))) 1.0))
        (Timeline|Timeline_0 PlayFromStart)))))

(fn ConstructionScript
  (bind _doormesh (Variables|Default|GetDoorMesh))
  (bind _door (Variables|Default|GetDoor))
  (bind _opendirection (Variables|Default|GetOpenDirection))
  (bind _door1 (Variables|Default|GetDoor1))
  (bind _returnvalue (Math|Float|SelectFloat 1.0 -1.0 _opendirection))
  (Components|StaticMesh|SetStaticMesh (Variables|Default|GetDoor) _doormesh)
  (Components|StaticMesh|SetStaticMesh (Variables|Default|GetDoor1) _doormesh)
  (if (Variables|Default|GetOpened)
    (Transformation|SetRelativeLocationAndRotation _door (Variables|/Script/Engine.SceneComponent|GetRelativeLocation _door) (Math|Rotator|MakeRotator 0.0 0.0 (* _returnvalue 1.1e+02)) false false)
    (Transformation|SetRelativeLocationAndRotation _door1 (Variables|/Script/Engine.SceneComponent|GetRelativeLocation _door1) (Math|Rotator|MakeRotator 0.0 0.0 (* _returnvalue -2.9e+02)) false false)))

(fn WithinInteractionDistance
  (params (Distance :type Float%20%28double-precision%29))
  (return (<= (Math|Vector|DotProduct (Math|Vector|VectorGetAbs (- (Transformation|GetActorLocation (Game|Player|GetPlayerPawn 0)) (Transformation|GetActorLocation))) "1.000000,1.000000,1.000000") Distance)))

(fn CheckKeys
  (bind _asbp_first_person_character (Utilities|Casting|CastToBP_FirstPersonCharacter (Game|Player|GetPlayerPawn 0)))
  (bind (_array_element _array_index) (Utilities|Array|ForEachLoopwithBreak (Variables|/Game/FirstPerson/Blueprints/BP_FirstPersonCharacter.BP_FirstPersonCharacter_C|GetKeys _asbp_first_person_character) :!label _label)
    (:LoopBody
      (if (== (Variables|Default|GetDoor_Id) _array_element)
        (Utilities|Array|RemoveIndex (Variables|/Game/FirstPerson/Blueprints/BP_FirstPersonCharacter.BP_FirstPersonCharacter_C|GetKeys _asbp_first_person_character) _array_index)
        (Variables|Default|SetUnlocked true)
        (goto _label Break)))))

(fn SetDoor
  (bind _opendirection (Variables|Default|GetOpenDirection))
  (bind _doormesh (Variables|Default|GetDoorMesh))
  (bind _door (Variables|Default|GetDoor))
  (bind _door1 (Variables|Default|GetDoor1))
  (bind _door1_2 (Variables|Default|GetDoor1))
  (bind _door_2 (Variables|Default|GetDoor))
  (bind _returnvalue (Math|Float|SelectFloat 1.0 -1.0 _opendirection))
  (Components|StaticMesh|SetStaticMesh (Variables|Default|GetDoor) _doormesh)
  (Components|StaticMesh|SetStaticMesh (Variables|Default|GetDoor1) _doormesh)
  (if (Variables|Default|GetOpened)
    (Transformation|SetRelativeLocationAndRotation _door_2 (Variables|/Script/Engine.SceneComponent|GetRelativeLocation _door_2) (Math|Rotator|MakeRotator 0.0 0.0 (* _returnvalue 1.1e+02)) false false)
    (Transformation|SetRelativeLocationAndRotation _door1 (Variables|/Script/Engine.SceneComponent|GetRelativeLocation _door1) (Math|Rotator|MakeRotator 0.0 0.0 (* _returnvalue -2.9e+02)) false false)
    (else
      (Transformation|SetRelativeLocationAndRotation _door (Variables|/Script/Engine.SceneComponent|GetRelativeLocation _door) (Math|Rotator|MakeRotator 0.0 0.0 0.0) false false)
      (Transformation|SetRelativeLocationAndRotation _door1_2 (Variables|/Script/Engine.SceneComponent|GetRelativeLocation _door1_2) (Math|Rotator|MakeRotator 0.0 0.0 1.8e+02) false false))))