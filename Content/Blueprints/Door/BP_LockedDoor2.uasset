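; BP_LockedDoor2 is a locked door that opens when the nearby player carries a key matching its DoorId.
; HighLight gates interaction using a Manhattan-distance check and shows an open prompt until the door opens.
; PickUp consumes the matching key from BP_FirstPersonCharacter, then a timeline swings the door's yaw with sound.
; Without a key, a DoOnce-guarded branch briefly shows a locked notice and message widget with a locked sound.
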(event EventHighLight
  (if (CallFunction|WithinInteractionDistance (Variables|Default|GetInteraction_Distance))
    (if (not (Variables|Default|GetOpened))
      (Rendering|SetVisibility (Variables|Default|GetOpenDoorNotice) true false)
      (Variables|Default|SetIs_Player_Nearby true))
    (else
      (Rendering|SetVisibility (Variables|Default|GetOpenDoorNotice) false false)
      (Variables|Default|SetIs_Player_Nearby false))))

(event EventRemoveHighLight
  (Rendering|SetVisibility (Variables|Default|GetOpenDoorNotice) false false)
  (Variables|Default|SetIs_Player_Nearby false))

(event EventPickUp
  (bind _returnvalue (Transformation|GetActorLocation))
  (bind _door (Variables|Default|GetDoor))
  (bind _doorlockednotice (Variables|Default|GetDoorLockedNotice))
  (bind _returnvalue_2 (Transformation|GetRelativeTransform _door))
  (if (Variables|Default|GetIs_Player_Nearby)
    (Variables|Default|SetAttemped true)
    (CallFunction|CheckKeys)
    (if (Variables|Default|GetUnlocked)
      (Audio|PlaySoundatLocation "/Game/Audio/door_open3.door_open3" _returnvalue "0, 0, 0" 1.0 1.0 0.0 0 0 0 0)
      (bind _open (Timeline|Open Play)
        (:Update
          (Transformation|SetRelativeLocationAndRotation (Variables|Default|GetDoor) (.location _returnvalue_2) (Math|Rotator|MakeRotator (.roll (.rotation _returnvalue_2)) (.pitch (.rotation _returnvalue_2)) _open) false false)
          (Variables|Default|SetOpened true)
          (Rendering|SetVisibility (Variables|Default|GetOpenDoorNotice) false false)))
      (else
        (Utilities|FlowControl|DoOnce false :!label _label
          (:Completed
            (bind _returnvalue_3 (UserInterface|CreateWidget "/Game/Blueprints/Door/WDJ_Message.WDJ_Message_C"))
            (UserInterface|Viewport|AddtoViewport _returnvalue_3 0)
            (Audio|PlaySoundatLocation "/Game/Audio/door_locked1.door_locked1" _returnvalue "0, 0, 0" 1.0 1.0 0.0 0 0 0 0)
            (Rendering|SetVisibility _doorlockednotice true false)
            (Utilities|FlowControl|Delay 1.0)
            (Rendering|SetVisibility _doorlockednotice false false)
            (Utilities|FlowControl|Delay 2.0)
            (Widget|RemovefromParent _returnvalue_3)
            (goto _label Reset)))))))

(fn ConstructionScript)

(fn WithinInteractionDistance
  (params (Distance :type Float%20%28double-precision%29))
  (return (<= (Math|Vector|DotProduct (Math|Vector|VectorGetAbs (- (Transformation|GetActorLocation (Game|Player|GetPlayerPawn 0)) (Transformation|GetActorLocation))) "1.000000,1.000000,1.000000") Distance)))

(fn CheckKeys
  (bind _asbp_first_person_character (Utilities|Casting|CastToBP_FirstPersonCharacter (Game|Player|GetPlayerPawn 0)))
  (bind _array_element (Utilities|Array|ForEachLoopwithBreak (Variables|/Game/FirstPerson/Blueprints/BP_FirstPersonCharacter.BP_FirstPersonCharacter_C|GetKeys _asbp_first_person_character) :!label _label)
    (:LoopBody
      (if (== (Variables|Default|GetDoor_Id) _array_element)
        (bind _returnvalue (Utilities|Array|RemoveItem (Variables|/Game/FirstPerson/Blueprints/BP_FirstPersonCharacter.BP_FirstPersonCharacter_C|GetKeys _asbp_first_person_character) _array_element))
        (Variables|Default|SetUnlocked _returnvalue)
        (goto _label Break)))))