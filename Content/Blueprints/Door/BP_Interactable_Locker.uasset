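; BP_Interactable_Locker is an interactable locker that lowers the player's panic while they are inside with the doors closed.
; PickUp plays a sound and swings both doors through the Open timeline, reversing it to close.
; HighLight shows an open/close prompt widget within interaction distance, measured as summed axis offsets, and enables PickUp.
; Box overlap starts a Delay-based polling loop that reduces the character's PanicValue while closed and overlapped.
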(event OnComponentBeginOverlap(Box)
  (params (OverlappedComponent :type Primitive%20Component%20Object%20Reference) (OtherActor :type Actor%20Object%20Reference) (OtherComp :type Primitive%20Component%20Object%20Reference) (OtherBodyIndex :type Integer) (bFromSweep :type Boolean) (SweepResult :type Hit%20Result%20Structure%20%28by%20ref%29))
  (bind _returnvalue (Game|Player|GetPlayerPawn 0))
  ;[1 1 1] Lower Panic
  (Variables|Default|SetOverlap true)
  (if (== OtherActor _returnvalue)
    (bind _asbp_first_person_character (Utilities|Casting|CastToBP_FirstPersonCharacter _returnvalue))
    (if (Variables|Default|GetOpened) :!label _label
      (Utilities|FlowControl|Delay 0.2 :!label _label_2)
      (goto _label)
      (elif (Variables|Default|GetOverlap)
        (Variables|/Game/FirstPerson/Blueprints/BP_FirstPersonCharacter.BP_FirstPersonCharacter_C|SetPanic_Value _asbp_first_person_character (- (Variables|/Game/FirstPerson/Blueprints/BP_FirstPersonCharacter.BP_FirstPersonCharacter_C|GetPanic_Value _asbp_first_person_character) 0.5))
        (goto _label_2)))))

(event OnComponentEndOverlap(Box)
  (params (OverlappedComponent :type Primitive%20Component%20Object%20Reference) (OtherActor :type Actor%20Object%20Reference) (OtherComp :type Primitive%20Component%20Object%20Reference) (OtherBodyIndex :type Integer))
  ;[1 1 1] Lower Panic
  (if (== OtherActor (Game|Player|GetPlayerPawn 0))
    (Variables|Default|SetOverlap false)))

(event EventHighLight
  (if (CallFunction|WithinInteractionDistance (Variables|Default|GetInteraction_Distance))
    (Rendering|SetVisibility (Variables|Default|GetOpenDoorNotice) true false)
    (bind _returnvalue (UserInterface|CreateWidget "/Game/Blueprints/Door/WBP_OpenDoor.WBP_OpenDoor_C"))
    (if (Variables|Default|GetOpened)
      (Variables|/Game/Blueprints/Door/WBP_OpenDoor.WBP_OpenDoor_C|SetPrompt _returnvalue "Close Locker [E]")
      (else
        (Variables|/Game/Blueprints/Door/WBP_OpenDoor.WBP_OpenDoor_C|SetPrompt _returnvalue "Open Locker [E]")))
    (UserInterface|SetWidget (Variables|Default|GetOpenDoorNotice) _returnvalue)
    (Variables|Default|SetIs_Player_Nearby true)
    (else
      (Rendering|SetVisibility (Variables|Default|GetOpenDoorNotice) false false)
      (Variables|Default|SetIs_Player_Nearby false))))

(event EventRemoveHighLight
  (Rendering|SetVisibility (Variables|Default|GetOpenDoorNotice) false false)
  (Variables|Default|SetIs_Player_Nearby false))

(event EventPickUp
  (bind _door (Variables|Default|GetDoor))
  (bind _door1 (Variables|Default|GetDoor1))
  (bind _returnvalue (Transformation|GetRelativeTransform _door))
  (bind _returnvalue_2 (Transformation|GetRelativeTransform _door1))
  (if (Variables|Default|GetIs_Player_Nearby)
    (Audio|PlaySoundatLocation "/Game/Audio/door_open2.door_open2" (Transformation|GetActorLocation) "0, 0, 0" 1.0 1.0 0.0 "/Game/Audio/NewSoundAttenuation.NewSoundAttenuation" 0 0 0)
    (if (Variables|Default|GetOpened)
      (Variables|Default|SetOpened false)
      (bind (_direction _open _open2) (Timeline|Open Reverse)
        (:Update
          (Transformation|SetRelativeLocationAndRotation _door (.location _returnvalue) (Math|Rotator|MakeRotator (.roll (.rotation _returnvalue)) (.pitch (.rotation _returnvalue)) _open) false false)
          (Transformation|SetRelativeLocationAndRotation _door1 (.location _returnvalue_2) (Math|Rotator|MakeRotator (.roll (.rotation _returnvalue_2)) (.pitch (.rotation _returnvalue_2)) _open2) false false)))
      (else
        (Variables|Default|SetOpened true)
        (Timeline|Open Play)))))

(fn ConstructionScript)

(fn WithinInteractionDistance
  (params (Distance :type Float%20%28double-precision%29))
  (return (<= (Math|Vector|DotProduct (Math|Vector|VectorGetAbs (- (Transformation|GetActorLocation (Game|Player|GetPlayerPawn 0)) (Transformation|GetActorLocation))) "1.000000,1.000000,1.000000") Distance)))