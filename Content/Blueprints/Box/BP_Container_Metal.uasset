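; Interactable metal container whose hinged Pivot swings open and closed on a timeline with sound, optionally locked behind a key.
; HighLight and RemoveHighLight toggle a prompt widget, using a Manhattan-distance range check to enable interaction.
; PickUp toggles the door or, if locked, uses a matching DoorId key from the player's inventory, otherwise showing a timed locked message.
; The construction script pre-rotates containers flagged Opened.
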(event EventHighLight
  ;[1 1 1] Show Door Prompt
  (if (CallFunction|WithinInteractionDistance (Variables|Default|GetInteraction_Distance))
    (Rendering|SetVisibility (Variables|Default|GetOpenDoorNotice) true false)
    (bind _returnvalue (UserInterface|CreateWidget "/Game/Blueprints/Door/WBP_OpenDoor.WBP_OpenDoor_C"))
    (if (Variables|Default|GetDisplayLocked)
      (Variables|/Game/Blueprints/Door/WBP_OpenDoor.WBP_OpenDoor_C|SetPrompt _returnvalue "Locked")
      (elif (Variables|Default|GetOpened)
        (Variables|/Game/Blueprints/Door/WBP_OpenDoor.WBP_OpenDoor_C|SetPrompt _returnvalue "Close Container [E]")
        (else
          (Variables|/Game/Blueprints/Door/WBP_OpenDoor.WBP_OpenDoor_C|SetPrompt _returnvalue "Open Container [E]"))))
    (UserInterface|SetWidget (Variables|Default|GetOpenDoorNotice) _returnvalue)
    (Variables|Default|SetIs_Player_Nearby true)))

(event EventRemoveHighLight
  ;[1 1 1] Show Door Prompt
  (Rendering|SetVisibility (Variables|Default|GetOpenDoorNotice) false false)
  (Variables|Default|SetIs_Player_Nearby false))

(event EventPickUp
  (bind _returnvalue (Transformation|GetActorLocation))
  (bind _pivot (Variables|Default|GetPivot))
  ;[1 1 1] Open Door and Check Key
  (if (Variables|Default|GetIs_Player_Nearby)
    (if (Variables|Default|GetUnlocked)
      (Utilities|FlowControl|DoOnce false :!label _label
        (:Completed
          (if (Variables|Default|GetOpened)
            (Audio|PlaySoundatLocation 0 _returnvalue "0, 0, 0" 1.0 1.0 0.0 "/Game/Audio/NewSoundAttenuation.NewSoundAttenuation" 0 0 0)
            (Variables|Default|SetOpened false)
            (bind _open (Timeline|Open ReverseFromEnd)
              (:Update
                (Transformation|SetRelativeLocationAndRotation _pivot (Variables|/Script/Engine.SceneComponent|GetRelativeLocation _pivot) (Math|Rotator|MakeRotator 0.0 _open 0.0) false false))
              (:Finished
                (goto _label Reset)))
            (else
              (Audio|PlaySoundatLocation 0 _returnvalue "0, 0, 0" 1.0 1.0 0.0 "/Game/Audio/NewSoundAttenuation.NewSoundAttenuation" 0 0 0)
              (Variables|Default|SetOpened true :!label _label_2)
              (Timeline|Open PlayFromStart)))))
      (else
        (CallFunction|CheckKeys)
        (if (Variables|Default|GetUnlocked)
          (Audio|PlaySoundatLocation "/Game/Audio/door_open3.door_open3" _returnvalue "0, 0, 0" 1.0 1.0 0.0 "/Game/Audio/NewSoundAttenuation.NewSoundAttenuation" 0 0 0)
          (goto _label_2)
          (else
            ;[1 1 1] Handle Locked Prompts
            (Utilities|FlowControl|DoOnce false :!label _label_3
              (:Completed
                (Variables|Default|SetDisplayLocked true)
                (bind _returnvalue_2 (UserInterface|CreateWidget "/Game/Blueprints/Door/WDJ_Message.WDJ_Message_C"))
                (Variables|/Game/Blueprints/Door/WDJ_Message.WDJ_Message_C|SetMessage _returnvalue_2 (Variables|Default|GetDoor%20Locked%20Message))
                (UserInterface|Viewport|AddtoViewport _returnvalue_2 0)
                (Audio|PlaySoundatLocation 0 (Transformation|GetActorLocation) "0, 0, 0" 1.0 1.0 0.0 "/Game/Audio/NewSoundAttenuation.NewSoundAttenuation" 0 0 0)
                (Utilities|FlowControl|Delay 2.0)
                (Widget|RemovefromParent _returnvalue_2)
                (Variables|Default|SetDisplayLocked false)
                (goto _label_3 Reset)))))))))

(fn ConstructionScript
  (bind _pivot (Variables|Default|GetPivot))
  (if (Variables|Default|GetOpened)
    (Transformation|SetRelativeLocationAndRotation _pivot (Variables|/Script/Engine.SceneComponent|GetRelativeLocation _pivot) (Math|Rotator|MakeRotator 0.0 -95.0 0.0) false false)))

(fn WithinInteractionDistance
  (params (Distance :type Float%20%28double-precision%29))
  (return (<= (Math|Vector|DotProduct (Math|Vector|VectorGetAbs (- (Transformation|GetActorLocation (Game|Player|GetPlayerPawn 0)) (Transformation|GetActorLocation))) "1.000000,1.000000,1.000000") Distance)))

(fn CheckKeys
  (bind _door_id (Variables|Default|GetDoor_Id))
  (bind _asbp_first_person_character (Utilities|Casting|CastToBP_FirstPersonCharacter (Game|Player|GetPlayerPawn 0)))
  (bind _havekey (Default|HaveKey (Variables|/Game/FirstPerson/Blueprints/BP_FirstPersonCharacter.BP_FirstPersonCharacter_C|GetBPC_Inventory_Component _asbp_first_person_character) _door_id))
  (if _havekey
    (bind _successful (Default|UseKey (Variables|/Game/FirstPerson/Blueprints/BP_FirstPersonCharacter.BP_FirstPersonCharacter_C|GetBPC_Inventory_Component _asbp_first_person_character) _door_id))
    (Variables|Default|SetUnlocked _successful)))