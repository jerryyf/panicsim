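; A standalone world marker that shows the player's distance to it and hides once the player reaches it.
; Its widget receives a colour on BeginPlay and a distance in whole metres every Tick, measured from the player character.
; When the player pawn overlaps the box, it sets an Overlapped flag and hides its own widget plus those of its linked BP_Side_Marker actors.
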(event OnComponentBeginOverlap(Box)
  (params (OverlappedComponent :type Primitive%20Component%20Object%20Reference) (OtherActor :type Actor%20Object%20Reference) (OtherComp :type Primitive%20Component%20Object%20Reference) (OtherBodyIndex :type Integer) (bFromSweep :type Boolean) (SweepResult :type Hit%20Result%20Structure%20%28by%20ref%29))
  (if (== OtherActor (Game|Player|GetPlayerPawn 0))
    (Variables|Default|SetOverlapped true)
    (Rendering|SetVisibility (Variables|Default|GetMarkerWidget) false false)
    (for _array_element (Variables|Default|GetSide%20Markers)
      (bind _asbp_side_marker (Utilities|Casting|CastToBP_Side_Marker _array_element))
      (Rendering|SetVisibility (Variables|/Game/Blueprints/Markers/BP_Side_Marker.BP_Side_Marker_C|GetSideMarkerWidget _asbp_side_marker) false false))))

(event EventBeginPlay
  (Class|BPIMarker|SetColour(Message) (UserInterface|GetUserWidgetObject (Variables|Default|GetMarkerWidget)) (Variables|Default|Getcolour)))

(event Collision|EventActorBeginOverlap
  (params (OtherActor :type Actor%20Object%20Reference)))

(event EventTick
  (params (DeltaSeconds :type Float%20%28single-precision%29))
  (Class|BPIMarker|UpdateDistance(Message) (UserInterface|GetUserWidgetObject (Variables|Default|GetMarkerWidget)) (Utilities|Text|ToText(String) (Utilities|String|Append (Utilities|String|ToString(Integer) (Math|Float|Truncate (/ (Math|Vector|Distance(Vector) (Transformation|GetActorLocation) (Transformation|GetActorLocation (Game|GetPlayerCharacter 0))) 1e+02))) "m"))))

(fn ConstructionScript)