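; BP_Marker_set steps through an ordered array of BP_Marker objects, showing the next marker as the current one is overlapped.
; Each tick it checks the marker at the current index and, once that marker is overlapped, hides it and advances the index.
; A DoOnce, reset on each advance, turns the new current marker visible a single time instead of every frame.
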(event EventTick
  (params (DeltaSeconds :type Float%20%28single-precision%29))
  (bind _asbp_marker (Utilities|Casting|CastToBP_Marker (Utilities|Array|Get(acopy) (Variables|Default|GetMarkers) (Variables|Default|GetNext%20Element%20Index))))
  (if (Variables|/Game/Blueprints/Markers/BP_Marker.BP_Marker_C|GetOverlapped _asbp_marker)
    (Variables|Default|SetNext%20Element%20Index (+ (Variables|Default|GetNext%20Element%20Index) 1))
    (Default|SetVisiblityOff _asbp_marker)
    (goto _label Reset)
    (else
      (Utilities|FlowControl|DoOnce false :!label _label
        (:Completed
          (Default|SetVisibilityon _asbp_marker))))))

(fn ConstructionScript)