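; BP_Getaway is a car actor, filed under PoliceCar, with switchable lights and an engine idle sound.
; ToggleLighton and ToggleLightOff set a shared brightness value to full or zero, then apply it as the intensity of two point lights and two spot lights.
; On BeginPlay it plays the idle sound with attenuation at the actor's location, so the sound is not attached to the car.
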(event EventToggleLighton
  (Variables|Default|SetCurrentBrightness 5e+03)
  (Rendering|Components|Light|SetIntensity (Variables|Default|GetPointLight) (stale EventToggleLightOff _output_get)))

(event EventToggleLightOff
  (bind _output_get (Variables|Default|SetCurrentBrightness 0.0))
  (Rendering|Components|Light|SetIntensity (Variables|Default|GetPointLight) _output_get))

(event EventBeginPlay
  (Audio|PlaySoundatLocation "/Game/Audio/car_idle.car_idle" (Transformation|GetActorLocation) "0, 0, 0" 1.0 1.0 0.0 "/Game/Audio/NewSoundAttenuation.NewSoundAttenuation" 0 0 0))

(fn ConstructionScript)