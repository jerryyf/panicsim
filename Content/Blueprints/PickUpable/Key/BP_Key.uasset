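; BP_Key is a key pickup that adds its KeyId to the first-person character's Keys and then destroys itself.
; HighLight highlights the key only within PickUpDistance of the player pawn, measured as a sum of absolute axis offsets (Manhattan distance) rather than straight-line length.
; Highlighting swaps the material and shows the name and pickup notice; RemoveHighLight reverts both.
; PickUp works only while the key is highlighted.
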(event EventHighLight
  (if (CallFunction|WithinPickUpDistance (Variables|Default|GetPickUp_Distance))
    (Variables|Default|SetHighlighted true)
    (Utilities|ChangeMaterial :!label _label)
    (else
      (Variables|Default|SetHighlighted false)
      (goto _label Normal))))

(event EventRemoveHighLight
  (Variables|Default|SetHighlighted false)
  (Utilities|ChangeMaterial) ; enters at Normal
)

(event EventPickUp
  (if (Variables|Default|GetHighlighted)
    (CallFunction|AddtoPlayer)))

(fn ConstructionScript)

(fn WithinPickUpDistance
  (params (Distance :type Float%20%28double-precision%29))
  (return (<= (Math|Vector|DotProduct (Math|Vector|VectorGetAbs (- (Transformation|GetActorLocation (Game|Player|GetPlayerPawn 0)) (Transformation|GetActorLocation))) "1.000000,1.000000,1.000000") Distance)))

(fn AddtoPlayer
  (bind _asbp_first_person_character (Utilities|Casting|CastToBP_FirstPersonCharacter (Game|Player|GetPlayerPawn 0)))
  (Utilities|Array|Add (Variables|/Game/FirstPerson/Blueprints/BP_FirstPersonCharacter.BP_FirstPersonCharacter_C|GetKeys _asbp_first_person_character) (Variables|Default|GetKey_Id))
  (Actor|DestroyActor))