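; BP_Bottle is a pickupable bottle that the first-person player can highlight and add to their inventory.
; HighLight checks Manhattan distance to the player, then a shared macro swaps the bottle material and toggles the name and pickup notice.
; PickUp works only while highlighted: with free storage it spawns a BP_Item carrying Name and Icon, plays a sound and destroys itself.
; A full inventory shows WBP_Inventory_Full instead.
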(event EventRemoveHighLight
  (Utilities|ChangeMaterial) ; enters at Normal
)

(event EventPickUp
  (if (Variables|Default|GetHighlighted)
    (CallFunction|AddtoPlayer)))

(event EventHighLight
  (if (CallFunction|WithinPickUpDistance (Variables|Default|GetPickUp_Distance))
    (Utilities|ChangeMaterial :!label _label)
    (else
      (goto _label Normal))))

(fn ConstructionScript)

(fn WithinPickUpDistance
  (params (Distance :type Float%20%28double-precision%29))
  (return (<= (Math|Vector|DotProduct (Math|Vector|VectorGetAbs (- (Transformation|GetActorLocation (Game|Player|GetPlayerPawn 0)) (Transformation|GetActorLocation))) "1.000000,1.000000,1.000000") Distance)))

(fn AddtoPlayer
  (bind _asbp_first_person_character (Utilities|Casting|CastToBP_FirstPersonCharacter (Game|Player|GetPlayerPawn 0)))
  (if (< (Utilities|Array|Length (Variables|/Game/FirstPerson/Blueprints/BP_FirstPersonCharacter.BP_FirstPersonCharacter_C|GetInventory _asbp_first_person_character)) (Variables|/Game/FirstPerson/Blueprints/BP_FirstPersonCharacter.BP_FirstPersonCharacter_C|GetStorage _asbp_first_person_character))
    (bind _returnvalue (Game|SpawnActorfromClass "/Game/Blueprints/PickUpable/BP_Item.BP_Item_C" (Transformation|GetActorTransform) "DontSpawnIfColliding" 0 0))
    (Variables|/Game/Blueprints/PickUpable/BP_Item.BP_Item_C|SetName _returnvalue (Variables|Default|GetName))
    (Variables|/Game/Blueprints/PickUpable/BP_Item.BP_Item_C|SetIcon _returnvalue (Variables|Default|GetIcon))
    (Utilities|Array|Add (Variables|/Game/FirstPerson/Blueprints/BP_FirstPersonCharacter.BP_FirstPersonCharacter_C|GetInventory _asbp_first_person_character) _returnvalue)
    (Audio|PlaySoundatLocation "/Game/SoundEffects/SoundCues/Pick_Up.Pick_Up" (Transformation|GetActorLocation) "0, 0, 0" 1.0 1.0 0.0 0 0 0 0)
    (Actor|DestroyActor)
    (else
      (bind _returnvalue_2 (UserInterface|CreateWidget "/Game/Blueprints/UI/Inventory/WBP_Inventory_Full.WBP_Inventory_Full_C"))
      (UserInterface|Viewport|AddtoViewport _returnvalue_2 0))))