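; BP_Panic_Area_Box is a trigger volume that steadily raises the player's panic while they stand inside it.
; On box overlap by the player pawn, it shows a WBP_Panic_Indicater widget and casts to BP_FirstPersonCharacter.
; A looping Delay increments PanicValue and calls PanicCheckMessage until the maximum is reached or the Overlap flag clears.
; Actor end overlap clears that flag and removes the widget.
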(event OnComponentBeginOverlap(Box)
  (params (OverlappedComponent :type Primitive%20Component%20Object%20Reference) (OtherActor :type Actor%20Object%20Reference) (OtherComp :type Primitive%20Component%20Object%20Reference) (OtherBodyIndex :type Integer) (bFromSweep :type Boolean) (SweepResult :type Hit%20Result%20Structure%20%28by%20ref%29))
  (if (== OtherActor (Game|Player|GetPlayerPawn 0))
    (Variables|Default|SetOverlap true)
    (bind _returnvalue (UserInterface|CreateWidget "/Game/Blueprints/Panic_Control/WBP_Panic_Indicater.WBP_Panic_Indicater_C"))
    (UserInterface|Viewport|AddtoViewport _returnvalue 0)
    (bind _asbp_first_person_character (Utilities|Casting|CastToBP_FirstPersonCharacter OtherActor))
    (if (Variables|Default|GetOverlap) :!label _label
      (if (< (Variables|/Game/FirstPerson/Blueprints/BP_FirstPersonCharacter.BP_FirstPersonCharacter_C|GetPanic_Value _asbp_first_person_character) (Variables|/Game/FirstPerson/Blueprints/BP_FirstPersonCharacter.BP_FirstPersonCharacter_C|GetMax_Panic_Value _asbp_first_person_character))
        (Variables|/Game/FirstPerson/Blueprints/BP_FirstPersonCharacter.BP_FirstPersonCharacter_C|SetPanic_Value _asbp_first_person_character (+ (Variables|/Game/FirstPerson/Blueprints/BP_FirstPersonCharacter.BP_FirstPersonCharacter_C|GetPanic_Value _asbp_first_person_character) 0.5))
        (Utilities|FlowControl|Delay 0.02)
        (Class|BPIPanicCheck|PanicCheck(Message) _asbp_first_person_character)
        (goto _label)))))

(event Collision|EventActorEndOverlap
  (params (OtherActor :type Actor%20Object%20Reference))
  (if (== OtherActor (Game|Player|GetPlayerPawn 0))
    (Variables|Default|SetOverlap false)
    (Widget|RemovefromParent (stale OnComponentBeginOverlap(Box) _returnvalue))))

(fn ConstructionScript)