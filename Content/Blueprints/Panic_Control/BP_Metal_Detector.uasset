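; BP_Metal_Detector is a hazard that reacts when the player carries a metal package.
; Entering WarningBox with that package type shows a WDJ_Message widget advising a package change, removed when an overlap with that box ends.
; Entering DetectBox with it applies damage to the player's BP_FirstPersonCharacter.
; Both boxes rely on CheckMetalPackage, which compares the character's PackageType against a single enum value.
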(event OnComponentBeginOverlap(DetectBox)
  (params (OverlappedComponent :type Primitive%20Component%20Object%20Reference) (OtherActor :type Actor%20Object%20Reference) (OtherComp :type Primitive%20Component%20Object%20Reference) (OtherBodyIndex :type Integer) (bFromSweep :type Boolean) (SweepResult :type Hit%20Result%20Structure%20%28by%20ref%29))
  (if (== (Game|Player|GetPlayerPawn 0) OtherActor)
    (if (CallFunction|CheckMetalPackage)
      (bind _asbp_first_person_character (Utilities|Casting|CastToBP_FirstPersonCharacter (Game|Player|GetPlayerPawn 0)))
      (Game|Damage|ApplyDamage _asbp_first_person_character 1.0 0 0))))

(event OnComponentBeginOverlap(WarningBox)
  (params (OverlappedComponent :type Primitive%20Component%20Object%20Reference) (OtherActor :type Actor%20Object%20Reference) (OtherComp :type Primitive%20Component%20Object%20Reference) (OtherBodyIndex :type Integer) (bFromSweep :type Boolean) (SweepResult :type Hit%20Result%20Structure%20%28by%20ref%29))
  (if (== (Game|Player|GetPlayerPawn 0) OtherActor)
    (if (CallFunction|CheckMetalPackage)
      (bind _returnvalue (UserInterface|CreateWidget "/Game/Blueprints/Door/WDJ_Message.WDJ_Message_C"))
      (Variables|/Game/Blueprints/Door/WDJ_Message.WDJ_Message_C|SetMessage _returnvalue "Metal detector here... I should change my package type")
      (UserInterface|Viewport|AddtoViewport _returnvalue 0))))

(event OnComponentEndOverlap(WarningBox)
  (params (OverlappedComponent :type Primitive%20Component%20Object%20Reference) (OtherActor :type Actor%20Object%20Reference) (OtherComp :type Primitive%20Component%20Object%20Reference) (OtherBodyIndex :type Integer))
  (if (Utilities|IsValid (stale OnComponentBeginOverlap(WarningBox) _returnvalue))
    (Widget|RemovefromParent (stale OnComponentBeginOverlap(WarningBox) _returnvalue))))

(fn ConstructionScript)

(fn CheckMetalPackage
  (bind _asbp_first_person_character (Utilities|Casting|CastToBP_FirstPersonCharacter (Game|Player|GetPlayerPawn 0)))
  (return (Utilities|Enum|Equal(Enum) (Variables|/Game/FirstPerson/Blueprints/BP_FirstPersonCharacter.BP_FirstPersonCharacter_C|GetPackage_Type _asbp_first_person_character) "NewEnumerator1")))