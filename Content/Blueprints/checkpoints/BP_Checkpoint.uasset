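; BP_Checkpoint is a one-shot checkpoint that saves the game when its Box is first overlapped.
; The overlap zeroes the player character's PanicValue, runs PanicCheck, calls SaveGame on BP_FirstPersonGameMode, then calls ShowCheckPointText.
; That event shows a BP_CheckPointReachedText widget with the checkpoint's CheckpointText and removes it after a short delay.
; The overlapping actor is not checked, so whatever triggers the Box first consumes the DoOnce.
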(event OnComponentBeginOverlap(Box)
  (params (OverlappedComponent :type Primitive%20Component%20Object%20Reference) (OtherActor :type Actor%20Object%20Reference) (OtherComp :type Primitive%20Component%20Object%20Reference) (OtherBodyIndex :type Integer) (bFromSweep :type Boolean) (SweepResult :type Hit%20Result%20Structure%20%28by%20ref%29))
  (Utilities|FlowControl|DoOnce false
    (:Completed
      (bind _asbp_first_person_character (Utilities|Casting|CastToBP_FirstPersonCharacter (Game|GetPlayerCharacter 0)))
      (Variables|/Game/FirstPerson/Blueprints/BP_FirstPersonCharacter.BP_FirstPersonCharacter_C|SetPanic_Value _asbp_first_person_character 0.0)
      (Default|PanicCheck _asbp_first_person_character)
      (bind _asbp_first_person_game_mode (Utilities|Casting|CastToBP_FirstPersonGameMode (Game|GetGameMode)))
      (Default|SaveGame _asbp_first_person_game_mode)
      (CallFunction|ShowCheckPointText))))

(event Custom|Show%20Check%20Point%20Text
  (Utilities|FlowControl|DoOnce false
    (:Completed
      (bind _returnvalue (UserInterface|CreateWidget "/Game/Blueprints/checkpoints/BP_CheckPointReachedText.BP_CheckPointReachedText_C"))
      (Variables|/Game/Blueprints/checkpoints/BP_CheckPointReachedText.BP_CheckPointReachedText_C|SetCheckpoint_text _returnvalue (Variables|Default|GetCheckpoint%20Text))
      (UserInterface|Viewport|AddtoViewport _returnvalue 0)
      (Utilities|FlowControl|Delay 3.0)
      (Widget|RemovefromParent _returnvalue))))

(fn ConstructionScript)